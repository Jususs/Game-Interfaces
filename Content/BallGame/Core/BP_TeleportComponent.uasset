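; BP_TeleportComponent is a scene component that lets its owning actor teleport to an aimed point.
; On BeginPlay it spawns a BP_TeleportTarget marker, shown when StartTeleport begins aiming.
; While aiming, Tick line-traces along the component's forward vector, projects the hit onto navigation and moves the marker there.
; EndTeleport stops aiming and, only on a trace hit, moves the owner there with a height offset and hides the marker.
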(event `self.ReceiveBeginPlay`
  (set `self.ActorToBeTeleported` (`self.GetOwner`))
  (bind _returnvalue (`|SpawnActorFromClass` "/Game/BallGame/BP_TeleportTarget.BP_TeleportTarget_C" (`KismetMathLibrary.MakeTransform` (0.0 0.0 0.0)) "Undefined" "OverrideRootScale" null null))
  (set `self.TargetActor` _returnvalue))

(event `self.ReceiveTick`
  (params (DeltaSeconds :type "Float (single-precision)"))
  (if (`self.bIsTeleporting`)
    (`self.DetectHitPoint`)))

(fn `DetectHitPoint`
  (bind _returnvalue (`self.K2_GetComponentLocation`))
  (bind (_outhit _returnvalue_2) (`KismetSystemLibrary.LineTraceSingle` _returnvalue (+ _returnvalue (* (`self.GetForwardVector`) (`self.Distance`))) "TraceTypeQuery1"))
  (bind _output_get (set `self.HitLocation` (`NavigationSystemV1.K2_ProjectPointToNavigation` (`.Location` (`GameplayStatics.BreakHitResult` _outhit)))))
  (bind _output_get_2 (set `self.bHitDetected` _returnvalue_2))
  (if _output_get_2
    (`Actor.K2_SetActorLocation` (`self.TargetActor`) _output_get false false)))

(fn `EndTeleport`
  (bind (_hitlocation_x _hitlocation_y _hitlocation_z) (`KismetMathLibrary.BreakVector` (`self.HitLocation`)))
  (set `self.bIsTeleporting` false)
  (if (`self.bHitDetected`)
    (`Actor.K2_SetActorLocation` (`self.ActorToBeTeleported`) (`KismetMathLibrary.MakeVector` _hitlocation_x _hitlocation_y (+ _hitlocation_z 90.212493)) false false)
    (`self.SetVisibility` (`/Game/BallGame/BP_TeleportTarget.Sphere` (`self.TargetActor`)) false false)))

(fn `StartTeleport`
  (set `self.bIsTeleporting` true)
  (`self.SetVisibility` (`/Game/BallGame/BP_TeleportTarget.Sphere` (`self.TargetActor`)) true false))